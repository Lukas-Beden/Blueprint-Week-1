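; Player controller that turns Enhanced Input actions into movement, look, run, crouch and jump for the controlled pawn.
; BeginPlay adds the IMC_Character mapping context.
; Move and look feed the pawn directly, with movement relative to control yaw.
; Run and crouch only call ChangeSpeed on the pawn cast to Player, with crouch leaving a lower speed on release than on press; jump uses the same cast.
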(event Input|EnhancedActionEvents|EnhancedInputActionIA_Move
  (params (ActionValue :type Vector%202D%20Structure) (ElapsedSeconds :type Float%20%28double-precision%29) (TriggeredSeconds :type Float%20%28double-precision%29) (InputAction :type Input%20Action%20Object%20Reference :default "/Game/Exercice1/Inputs/InputActions/IA_Move.IA_Move"))
  (bind _returnvalue (Pawn|GetControlRotation :!class /Script/Engine.Controller))
  (bind _returnvalue_2 (Pawn|GetControlledPawn))
  (Pawn|Input|AddMovementInput _returnvalue_2 (Math|Vector|GetRightVector (Math|Rotator|MakeRotator (.roll _returnvalue) 0.0 (.yaw _returnvalue))) (.x ActionValue) false)
  (Pawn|Input|AddMovementInput _returnvalue_2 (Math|Vector|GetForwardVector (Math|Rotator|MakeRotator 0.0 0.0 (.yaw (Pawn|GetControlRotation :!class /Script/Engine.Controller)))) (.y ActionValue) false))

(event Input|EnhancedActionEvents|EnhancedInputActionIA_Look
  (params (ActionValue :type Vector%202D%20Structure) (ElapsedSeconds :type Float%20%28double-precision%29) (TriggeredSeconds :type Float%20%28double-precision%29) (InputAction :type Input%20Action%20Object%20Reference :default "/Game/Exercice1/Inputs/InputActions/IA_Look.IA_Look"))
  (bind _returnvalue (Pawn|GetControlledPawn))
  (Pawn|Input|AddControllerYawInput _returnvalue (.x ActionValue))
  (Pawn|Input|AddControllerPitchInput _returnvalue (.y ActionValue)))

(event Input|EnhancedActionEvents|EnhancedInputActionIA_Run
  (params (ActionValue :type Boolean) (ElapsedSeconds :type Float%20%28double-precision%29) (TriggeredSeconds :type Float%20%28double-precision%29) (InputAction :type Input%20Action%20Object%20Reference :default "/Game/Exercice1/Inputs/InputActions/IA_Run.IA_Run"))
  (bind _returnvalue (Pawn|GetControlledPawn))
  (:Started
    (bind _asplayer (Utilities|Casting|CastToPlayer _returnvalue))
    (Default|ChangeSpeed _asplayer 9e+02))
  (:Completed
    (bind _asplayer_2 (Utilities|Casting|CastToPlayer _returnvalue))
    (Default|ChangeSpeed _asplayer_2 6e+02)))

(event Input|EnhancedActionEvents|EnhancedInputActionIA_Jump
  (params (ActionValue :type Boolean) (ElapsedSeconds :type Float%20%28double-precision%29) (TriggeredSeconds :type Float%20%28double-precision%29) (InputAction :type Input%20Action%20Object%20Reference :default "/Game/Exercice1/Inputs/InputActions/IA_Jump.IA_Jump"))
  (bind _returnvalue (Pawn|GetControlledPawn))
  (:Triggered
    (bind _asplayer (Utilities|Casting|CastToPlayer _returnvalue))
    (Character|Jump _asplayer))
  (:Completed
    (bind _asplayer_2 (Utilities|Casting|CastToPlayer _returnvalue))
    (Character|StopJumping _asplayer_2)))

(event Input|EnhancedActionEvents|EnhancedInputActionIA_Crouch
  (params (ActionValue :type Boolean) (ElapsedSeconds :type Float%20%28double-precision%29) (TriggeredSeconds :type Float%20%28double-precision%29) (InputAction :type Input%20Action%20Object%20Reference :default "/Game/Exercice1/Inputs/InputActions/IA_Crouch.IA_Crouch"))
  (bind _returnvalue (Pawn|GetControlledPawn))
  (:Started
    (bind _asplayer (Utilities|Casting|CastToPlayer _returnvalue))
    (Default|ChangeSpeed _asplayer 6e+02))
  (:Completed
    (bind _asplayer_2 (Utilities|Casting|CastToPlayer _returnvalue))
    (Default|ChangeSpeed _asplayer_2 3e+02)))

(event EventBeginPlay
  (bind _returnvalue (Game|GetPlayerController 0))
  (bind _returnvalue_2 (PlayerController|LocalPlayerSubsystems|GetEnhancedInputLocalPlayerSubsystem _returnvalue))
  (Utilities|IsValid _returnvalue_2
    (:Is%20Valid
      (Input|AddMappingContext _returnvalue_2 "/Game/Exercice1/Inputs/IMC_Character.IMC_Character" 0 "(bIgnoreAllPressedKeysUntilRelease=True,bForceImmediately=False,bNotifyUserSettings=False)"))))

(event Collision|EventActorBeginOverlap
  (params (OtherActor :type Actor%20Object%20Reference)))

(event EventTick
  (params (DeltaSeconds :type Float%20%28single-precision%29)))

(fn ConstructionScript)